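; NPC character that walks to a middle spot to face the player, then leaves along a pass or non-pass route.
; On BeginPlay it binds to the BP_TestGameMode new-NPC dispatcher for arrival and two BP_PlayerCharacter dispatchers for the exits.
; Each move uses AI MoveTo with hard-coded destinations and directly played idle or walk animations.
; Both exits start after a short delay and end by teleporting to the same reset point.
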(event `self.ReceiveBeginPlay`
  (bind _outactors (`GameplayStatics.GetAllActorsOfClass` "/Game/BP_TestGameMode.BP_TestGameMode_C"))
  (add `/Game/BP_TestGameMode.NewNPC` (`|GetArrayItem` _outactors) (delegate `StartMove_Event`))
  (bind _outactors_2 (`GameplayStatics.GetAllActorsOfClass` "/Game/Characters/Player/BP_PlayerCharacter.BP_PlayerCharacter_C"))
  (bind _output (`|GetArrayItem` _outactors_2))
  (add `/Game/Characters/Player/BP_PlayerCharacter.NewEventDispatcher_0` _output (delegate `EndMove_Event`))
  (add `/Game/Characters/Player/BP_PlayerCharacter.NewEventDispatcher_1` _output (delegate `BackMove_Event`)))

(event `StartMove_Event`
  ;[1 1 1] Move1:Go Mid
  (`|AIMoveTo` self (450.0 20.0 226.0) null
    (:`OnSuccess`
      (`self.K2_SetActorRotation` (`KismetMathLibrary.FindLookAtRotation` (`self.K2_GetActorLocation`) (`self.K2_GetActorLocation` (`GameplayStatics.GetPlayerCharacter` 0))))
      (`SkeletalMeshComponent.PlayAnimation` (`self.Mesh`) "/Game/Characters/Mannequins/Animations/Quinn/MF_Idle.MF_Idle" true))))

(event `EndMove_Event`
  ;[0.2135 1 0.1232] Move2:Pass
  (`KismetSystemLibrary.Delay` 1.5)
  (`SkeletalMeshComponent.PlayAnimation` (`self.Mesh`) "/Game/Characters/Mannequins/Animations/Quinn/MF_Walk_Fwd.MF_Walk_Fwd" true)
  (`|AIMoveTo` self (450.0 950.0 226.0) null
    (:`OnSuccess`
      (`self.K2_TeleportTo` (200.0 -610.0 226.0)))))

(event `BackMove_Event`
  ;[1 0.1643 0.2241] Move3:NonPass
  (`KismetSystemLibrary.Delay` 1.5)
  (`SkeletalMeshComponent.PlayAnimation` (`self.Mesh`) "/Game/Characters/Mannequins/Animations/Quinn/MF_Walk_Fwd.MF_Walk_Fwd" true)
  (`|AIMoveTo` self (100.0 -600.0 226.0) null
    (:`OnSuccess`
      (`self.K2_TeleportTo` (200.0 -610.0 226.0)))))

(fn `UserConstructionScript`)