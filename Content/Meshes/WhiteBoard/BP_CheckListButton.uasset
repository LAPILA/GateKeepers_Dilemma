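; BP_CheckListButton is a whiteboard actor that animates its mesh into place and then shows a checklist widget.
; On BeginPlay, a timeline lerps MainMesh from its current world location toward the Plane component's location.
; The same Update pin feeds a three-second Delay, after which it creates WBP_CheckList and adds it to the viewport.
; A cast to BP_PlayerCharacter and a branch are left unconnected.
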(event `self.ReceiveBeginPlay`
  (bind (_direction `_새_트랙_0`) (`Timeline|타임라인`)
    (:`Update`
      (`SceneComponent.K2_SetWorldLocation` (`self.MainMesh`) (`KismetMathLibrary.VLerp` (`SceneComponent.K2_GetComponentLocation` (`self.MainMesh`)) (`SceneComponent.K2_GetComponentLocation` (`self.Plane`)) `_새_트랙_0`) false false)
      (`KismetSystemLibrary.Delay` 3.0)
      (bind _returnvalue (`|CreateWidget` "/Game/UI/WBP_CheckList.WBP_CheckList_C"))
      (`UserWidget.AddToViewport` _returnvalue 0))))

(event `Key|LeftMouseButton`
  (params (Key :type "Key Structure")))

(fn `UserConstructionScript`
  (`parent.UserConstructionScript`))