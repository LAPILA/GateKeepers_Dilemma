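; Game mode that generates each new NPC's identity and passport data for what appears to be a document-inspection game.
; On the player's event dispatcher, it rolls probability-based error flags, then copies a random row from the current day's DataTable, with later days adding fields.
; For each flagged field it picks a random error value from that field's error DataTable, or inverts gender, then calls CallNewNPC.
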(event `self.ReceiveBeginPlay`
  (bind _outactors (`GameplayStatics.GetAllActorsOfClass` "/Game/Characters/Player/BP_PlayerCharacter.BP_PlayerCharacter_C"))
  (add `/Game/Characters/Player/BP_PlayerCharacter.NewEventDispatcher` (`|GetArrayItem` _outactors) (delegate `NewNPC_Event`)))

(event `NewNPC_Event`
  ;[1 1 1] DataSetting
  (`self.Random Error Func`)
  (`self.Random Data Table`)
  (`self.Data Settings`)
  (`self.NewNPC`))

(fn `Data Settings`
  (if (`self.bNameValid`)
    (bind _outrownames (`DataTableFunctionLibrary.GetDataTableRowNames` "/Game/Data/ErrorDB/DT_ErrorName.DT_ErrorName"))
    (bind _returnvalue (`|GetDataTableRow` "/Game/Data/ErrorDB/DT_ErrorName.DT_ErrorName" (`KismetArrayLibrary.Array_Random` _outrownames))
      (:`then`
        (set `self.ErrorName` (`.Name_2_3BD653BC473C3D56244EBBAC27DC3DC1` (break `/Game/Data/ErrorDB/DS_ErrorName` _returnvalue))))))
  (if (`self.bPVValid`)
    (bind _outrownames_2 (`DataTableFunctionLibrary.GetDataTableRowNames` "/Game/Data/ErrorDB/DT_ErrorPassport_validityperiod.DT_ErrorPassport_validityperiod"))
    (bind _returnvalue_2 (`|GetDataTableRow` "/Game/Data/ErrorDB/DT_ErrorPassport_validityperiod.DT_ErrorPassport_validityperiod" (`KismetArrayLibrary.Array_Random` _outrownames_2))
      (:`then`
        (set `self.ErrorPassport Validityperiod` (`.Passport_validityperiod_2_3EFD4E6B4BCE5393636E57BDA1923A6F` (break `/Game/Data/ErrorDB/DS_ErrorPassport_validityperiod` _returnvalue_2))))))
  (if (`self.bIDValid`)
    (bind _outrownames_3 (`DataTableFunctionLibrary.GetDataTableRowNames` "/Game/Data/ErrorDB/DT_ErrorID.DT_ErrorID"))
    (bind _returnvalue_3 (`|GetDataTableRow` "/Game/Data/ErrorDB/DT_ErrorID.DT_ErrorID" (`KismetArrayLibrary.Array_Random` _outrownames_3))
      (:`then`
        (set `self.Error Identity Number` (`.Identity_number_2_036DD33942CF4AC7C0046B87E4D47BE0` (break `/Game/Data/ErrorDB/DS_ErrorID` _returnvalue_3))))))
  (if (`self.bPNValid`)
    (bind _outrownames_4 (`DataTableFunctionLibrary.GetDataTableRowNames` "/Game/Data/ErrorDB/DT_Errorpassport_number.DT_Errorpassport_number"))
    (bind _returnvalue_4 (`|GetDataTableRow` "/Game/Data/ErrorDB/DT_Errorpassport_number.DT_Errorpassport_number" (`KismetArrayLibrary.Array_Random` _outrownames_4))
      (:`then`
        (set `self.Error Passport Number` (`.passport_number_3_2166FEF34475079F0BA8F38DC8B4AC0C` (break `/Game/Data/ErrorDB/DS_Errorpassport_number` _returnvalue_4))))))
  (if (`self.bGenderValid`)
    (set `self.ErrorGender` (not (`self.Gender`))))
  (if (`self.bBirthValid`)
    (bind _outrownames_5 (`DataTableFunctionLibrary.GetDataTableRowNames` "/Game/Data/ErrorDB/DT_ErrorBirthDate.DT_ErrorBirthDate"))
    (bind _returnvalue_5 (`|GetDataTableRow` "/Game/Data/ErrorDB/DT_ErrorBirthDate.DT_ErrorBirthDate" (`KismetArrayLibrary.Array_Random` _outrownames_5))
      (:`then`
        (set `self.Error Birth Date` (`.BirthDate_2_8582E4D348568D70CA2800AD45F87906` (break `/Game/Data/ErrorDB/DS_ErrorBirthDate` _returnvalue_5)))))))

(fn `Random Data Table`
  ;[1 1 1] Data Table Set by Day
  (switch `int` (+ (`self.Day`) -1)
    (:`Default`
      (bind _outrownames (`DataTableFunctionLibrary.GetDataTableRowNames` "/Game/Data/NormalDB/DT_Day1.DT_Day1" :!label _label))
      (bind _returnvalue (`|GetDataTableRow` "/Game/Data/NormalDB/DT_Day1.DT_Day1" (`KismetArrayLibrary.Array_Random` _outrownames))
        (:`then`
          (bind (_name _identity_number _passport_number _passport_validityperiod _gender _birthdate _residence _npc_type) (break `/Game/Data/NormalDB/DS_Day1` _returnvalue))
          (set `self.Name` _name)
          (set `self.Identity Number` _identity_number)
          (set `self.Passport Number` _passport_number)
          (set `self.Passport Validityperiod` _passport_validityperiod)
          (set `self.Gender` _gender)
          (set `self.Birth Date` _birthdate)
          (set `self.Residence` _residence)
          (set `self.Npc Type` _npc_type))))
    (:`0`
      (goto _label))
    (:`1`
      (bind _outrownames_2 (`DataTableFunctionLibrary.GetDataTableRowNames` "/Game/Data/NormalDB/DT_Day2.DT_Day2"))
      (bind _returnvalue_2 (`|GetDataTableRow` "/Game/Data/NormalDB/DT_Day2.DT_Day2" (`KismetArrayLibrary.Array_Random` _outrownames_2))
        (:`then`
          (bind (_name_2 _identity_number_2 _passport_number_2 _passport_validityperiod_2 _gender_2 _birthdate_2 _residence_2 _purpose _period_stay _stamp _npc_type_2) (break `/Game/Data/NormalDB/DS_Day2` _returnvalue_2))
          (set `self.Name` _name_2)
          (set `self.Identity Number` _identity_number_2)
          (set `self.Passport Number` _passport_number_2)
          (set `self.Passport Validityperiod` _passport_validityperiod_2)
          (set `self.Gender` _gender_2)
          (set `self.Birth Date` _birthdate_2)
          (set `self.Residence` _residence_2)
          (set `self.Npc Type` _npc_type_2)
          (set `self.Purpose` _purpose)
          (set `self.Period Stay` _period_stay)
          (set `self.Stamp` _stamp))))
    (:`2`
      (bind _outrownames_3 (`DataTableFunctionLibrary.GetDataTableRowNames` "/Game/Data/NormalDB/DT_Day3.DT_Day3"))
      (bind _returnvalue_3 (`|GetDataTableRow` "/Game/Data/NormalDB/DT_Day3.DT_Day3" (`KismetArrayLibrary.Array_Random` _outrownames_3))
        (:`then`
          (bind (_name_3 _identity_number_3 _passport_number_3 _passport_validityperiod_3 _gender_3 _birthdate_3 _residence_3 _purpose_2 _period_stay_2 _stamp_2 _npc_type_3) (break `/Game/Data/NormalDB/DS_Day3` _returnvalue_3))
          (set `self.Name` _name_3)
          (set `self.Identity Number` _identity_number_3)
          (set `self.Passport Number` _passport_number_3)
          (set `self.Passport Validityperiod` _passport_validityperiod_3)
          (set `self.Gender` _gender_3)
          (set `self.Birth Date` _birthdate_3)
          (set `self.Residence` _residence_3)
          (set `self.Npc Type` _npc_type_3)
          (set `self.Purpose` _purpose_2)
          (set `self.Period Stay` _period_stay_2)
          (set `self.Stamp` _stamp_2))))
    (:`3`
      (bind _outrownames_4 (`DataTableFunctionLibrary.GetDataTableRowNames` "/Game/Data/NormalDB/DT_Day4.DT_Day4"))
      (bind _returnvalue_4 (`|GetDataTableRow` "/Game/Data/NormalDB/DT_Day4.DT_Day4" (`KismetArrayLibrary.Array_Random` _outrownames_4))
        (:`then`
          (bind (_name_4 _identity_number_4 _passport_number_4 _passport_validityperiod_4 _gender_4 _birthdate_4 _residence_4 _purpose_3 _period_stay_3 _stamp_3 _diagnosis _npc_type_4) (break `/Game/Data/NormalDB/DS_Day4` _returnvalue_4))
          (set `self.Name` _name_4)
          (set `self.Identity Number` _identity_number_4)
          (set `self.Passport Number` _passport_number_4)
          (set `self.Passport Validityperiod` _passport_validityperiod_4)
          (set `self.Gender` _gender_4)
          (set `self.Birth Date` _birthdate_4)
          (set `self.Residence` _residence_4)
          (set `self.Npc Type` _npc_type_4)
          (set `self.Purpose` _purpose_3)
          (set `self.Period Stay` _period_stay_3)
          (set `self.Stamp` _stamp_3)
          (set `self.Diagnosis` _diagnosis))))
    (:`4`
      (bind _outrownames_5 (`DataTableFunctionLibrary.GetDataTableRowNames` "/Game/Data/NormalDB/DT_Day5.DT_Day5"))
      (bind _returnvalue_5 (`|GetDataTableRow` "/Game/Data/NormalDB/DT_Day5.DT_Day5" (`KismetArrayLibrary.Array_Random` _outrownames_5))
        (:`then`
          (bind (_name_5 _identity_number_5 _passport_number_5 _passport_validityperiod_5 _gender_5 _birthdate_5 _residence_5 _purpose_4 _period_stay_4 _stamp_4 _diagnosis_2 _npc_type_5) (break `/Game/Data/NormalDB/DS_Day5` _returnvalue_5))
          (set `self.Name` _name_5)
          (set `self.Identity Number` _identity_number_5)
          (set `self.Passport Number` _passport_number_5)
          (set `self.Passport Validityperiod` _passport_validityperiod_5)
          (set `self.Gender` _gender_5)
          (set `self.Birth Date` _birthdate_5)
          (set `self.Residence` _residence_5)
          (set `self.Npc Type` _npc_type_5)
          (set `self.Purpose` _purpose_4)
          (set `self.Period Stay` _period_stay_4)
          (set `self.Stamp` _stamp_4)
          (set `self.Diagnosis` _diagnosis_2))))))

(fn `Random Error Func`
  ;[1 1 1] SetErrorFunc by probabilities
  (`self.SetValidationProbabilities` (`self.Probability_Error`) (`self.Probability_Name`) (`self.Probability_ID`) (`self.Probability_PNP`) (`self.Probability_PVP`) (`self.Probability_Gender`) (`self.Probability_Birth`))
  (`self.ValidateRandomData`)
  (`self.DebugPrintValidationResults`))

(fn `UserConstructionScript`)